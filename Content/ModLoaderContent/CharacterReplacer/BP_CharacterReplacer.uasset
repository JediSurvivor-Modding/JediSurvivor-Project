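; Mod actor for the character replacer: opens its GUI and applies modded outfits to every actor of the selected character class.
; Parts spawn as skeletal mesh actors attached with master pose, tracked by actor and part ID, and recolored through dynamic material instances.
; It toggles original meshes' visibility and spawns a rotatable preview framed by a scene capture.
; An older Cal profile path remains, largely stubbed or unwired.
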(event `GetAllAssets`
  (bind _assets (`/Game/Mods/ModLoader/BlueprintLibraries/ModLoaderUtilities.GetAssetsInPaksByPath` true "/Game/Mods"))
  (bind _output_get (set `self.Assets` _assets)))

(event `Key|Period`
  (params (Key :type "Key Structure"))
  (:`Pressed`
    (bind _profiles (`self.Load Cal Outfits`))
    (for _array_element _profiles
      (bind (_outfitname _outfitauthor _description _tags _thumbnail _profileref _pants _undershirt _jacket _head _hair _facialhair) (break `/Game/ModLoaderContent/CharacterReplacer/Profiles/Struct_Outfit` _array_element))
      (`self.Set Active Profile` (make `/Game/ModLoaderContent/CharacterReplacer/Profiles/Struct_UserProfile` "" null _pants _undershirt _jacket _head _hair _facialhair))
      (`KismetSystemLibrary.PrintString` _outfitname))))

(event `self.ReceiveBeginPlay`
  (bind _returnvalue (`GameplayStatics.GetPlayerController` 0))
  (bind (_returnvalue_x _returnvalue_y) (`KismetMathLibrary.BreakVector` (`self.K2_GetActorLocation` (`GameplayStatics.GetPlayerCharacter` 0))))
  (bind _returnvalue_2 (`|CreateWidget` "/Game/ModLoaderContent/CharacterReplacer/GUI/GUI_CharacterReplacer.GUI_CharacterReplacer_C" null self))
  (set `/Game/ModLoaderContent/UI/OutfitBrowser/Master_OutfitBrowser.CharacterReplacer` self (`/Game/ModLoaderContent/CharacterReplacer/GUI/GUI_CharacterReplacer.Master_OutfitBrowser` _returnvalue_2))
  (`UserWidget.AddToViewport` _returnvalue_2 0)
  (`WidgetBlueprintLibrary.SetInputMode_UIOnlyEx` _returnvalue _returnvalue_2)
  (set `PlayerController.bShowMouseCursor` true _returnvalue)
  (`MovementComponent.SetUpdatedComponent` (`self.RotatingMovement`) (`self.PreviewBase`))
  (`self.K2_SetActorLocation` (`KismetMathLibrary.MakeVector` _returnvalue_x _returnvalue_y (+ 0.0 (`self.Height`))) false true)
  (`self.UpdateMeshPreview` null))

(event `PrintToModLoader`
  (params (Message :type String))
  (`KismetSystemLibrary.PrintString` Message))

(event `UpdateCurrentCharacterClass`
  (params (Character :type "/Game/ModLoaderContent/CharacterReplacer/Profiles/Character/Enum_Character Enum" :default "NewEnumerator3") (CharacterClass :type "Character Class Reference"))
  (bind (_value _returnvalue) (`BlueprintMapLibrary.Map_Find` (`self.CharacterEnumToClass`) Character))
  (set `self.CurrentCharacterEnum` Character)
  (if _returnvalue
    (set `self.CurrentCharacterClass` _value)
    (else
      (set `self.CurrentCharacterClass` CharacterClass)))
  (`self.UpdateMeshPreview` null))

(event `self.ReceiveTick`
  (params (DeltaSeconds :type "Float (single-precision)")))

(fn `ApplyColor`
  (params (Color :type "/Game/ModLoaderContent/CharacterReplacer/Profiles/ColorProfile Class Reference") (Part :type "/Game/ModLoaderContent/CharacterReplacer/Profiles/Struct_Part Structure") (Outfit :type "/Game/ModLoaderContent/CharacterReplacer/Profiles/OutfitProfile Object Reference"))
  (`self.ResetColor` Part Outfit)
  (bind _outactors (`GameplayStatics.GetAllActorsOfClass` (`self.CurrentCharacterClass`)))
  (for _array_element _outactors
    (bind (_value _returnvalue) (`BlueprintMapLibrary.Map_Find` (`self.AddonMeshes`) (`KismetStringLibrary.Concat_StrStr` (`KismetSystemLibrary.GetObjectName` _array_element) (`/Game/ModLoaderContent/CharacterReplacer/Profiles/OutfitProfile.GetPartID` Outfit Part))))
    (if _returnvalue
      (for _array_element_2 (`.Parts` (defaults `Object` Color))
        (bind (_partname _materials) (break `/Game/ModLoaderContent/CharacterReplacer/Profiles/Struct_PartRetexture` _array_element_2))
        (if (== _partname (`.PartName_5_7666BC5344FF1AEE5B4442AF7394D2F7` (break `/Game/ModLoaderContent/CharacterReplacer/Profiles/Struct_Part` Part)))
          (for _array_element_3 _materials
            (bind _skeletalmeshcomponent (`SkeletalMeshActor.SkeletalMeshComponent` _value))
            (bind (_materialslotname _textures) (break `/Game/ModLoaderContent/CharacterReplacer/Profiles/Struct_Material` _array_element_3))
            (bind _returnvalue_2 (`MeshComponent.GetMaterialIndex` _skeletalmeshcomponent _materialslotname))
            (bind _returnvalue_3 (`PrimitiveComponent.CreateDynamicMaterialInstance` _skeletalmeshcomponent _returnvalue_2 (`PrimitiveComponent.GetMaterial` _skeletalmeshcomponent _returnvalue_2) _materialslotname))
            (for _array_element_4 _textures
              (bind (_parametername _texture) (break `/Game/ModLoaderContent/CharacterReplacer/Profiles/Struct_Texture` _array_element_4))
              (`MaterialInstanceDynamic.SetTextureParameterValue` _returnvalue_3 _parametername _texture)))
          (`/Game/ModLoaderContent/CharacterReplacer/Profiles/OutfitProfile.OnPartColorApplied` Outfit Part Color))))))

(fn `EquipPart`
  (params (Part :type "/Game/ModLoaderContent/CharacterReplacer/Profiles/Struct_Part Structure") (Outfit :type "/Game/ModLoaderContent/CharacterReplacer/Profiles/OutfitProfile Object Reference"))
  (locals (L_CurrentLoopMesh :type "SkinnedMeshComponent Object Reference"))
  (bind (_mesh _partname _parttype _replace) (break `/Game/ModLoaderContent/CharacterReplacer/Profiles/Struct_Part` Part))
  (bind _l_currentloopmesh (`local.L_CurrentLoopMesh`))
  (`/Engine/EditorBlueprintResources/StandardMacros.IsValid` _mesh
    (:`Is Valid`
      (bind _outactors (`GameplayStatics.GetAllActorsOfClass` (`self.CurrentCharacterClass`)))
      (for _array_element _outactors
        (set `local.L_CurrentLoopMesh` (`Character.Mesh` _array_element))
        (`|ExecutionSequence`
          (:`then_0`
            (if _replace
              _
              (else
                _))
            (bind _returnvalue (`|SpawnActorFromClass` "/Script/Engine.SkeletalMeshActor" (`self.GetTransform` _array_element) "AlwaysSpawn" "OverrideRootScale" null null))
            (`BlueprintMapLibrary.Map_Add` (`self.AddonMeshes`) (`KismetStringLibrary.Concat_StrStr` (`KismetSystemLibrary.GetObjectName` _array_element) (`/Game/ModLoaderContent/CharacterReplacer/Profiles/OutfitProfile.GetPartID` Outfit Part)) _returnvalue)
            (`PrimitiveComponent.SetCollisionEnabled` (`SkeletalMeshActor.SkeletalMeshComponent` _returnvalue) "NoCollision")
            (`self.K2_AttachToComponent` _returnvalue _l_currentloopmesh "None" "SnapToTarget" "SnapToTarget" "SnapToTarget" true)
            (bind _skeletalmeshcomponent (`SkeletalMeshActor.SkeletalMeshComponent` _returnvalue))
            (`SkinnedMeshComponent.SetSkinnedAssetAndUpdate` _skeletalmeshcomponent _mesh false)
            (`SkinnedMeshComponent.SetLeaderPoseComponent` _skeletalmeshcomponent _l_currentloopmesh false))))
      (`/Game/ModLoaderContent/CharacterReplacer/Profiles/OutfitProfile.OnPartEquipped` Outfit Outfit Part)
      (`self.OnAnyPartAdded` Outfit Part _replace)
      (`KismetArrayLibrary.Array_AddUnique` (`self.EquippedOutfits`) Outfit))))

(fn `GetFacialRig`
  (params (RsCharacter :type "Character Object Reference"))
  (returns (face :type "SkeletalMeshComponent Object Reference"))
  (bind _asbp_hero (cast `/Game/Characters/Hero/Logic/BP_Hero` RsCharacter))
  (return (`/Game/Characters/Hero/Logic/BP_Hero.face` _asbp_hero)))

(fn `Hide Parts`
  (params (Pants :type "/Game/ModLoaderContent/CharacterReplacer/Profiles/Struct_OutfitPart Structure") (UnderShirt :type "/Game/ModLoaderContent/CharacterReplacer/Profiles/Struct_OutfitPart Structure") (Jacket :type "/Game/ModLoaderContent/CharacterReplacer/Profiles/Struct_OutfitPart Structure") (Head :type "/Game/ModLoaderContent/CharacterReplacer/Profiles/Struct_OutfitPart Structure") (Hair :type "/Game/ModLoaderContent/CharacterReplacer/Profiles/Struct_OutfitPart Structure") (`Facial Hair` :type "/Game/ModLoaderContent/CharacterReplacer/Profiles/Struct_OutfitPart Structure"))
  (bind _face (`self.GetFacialRig` (`GameplayStatics.GetPlayerCharacter` 0)))
  (`SceneComponent.SetVisibility` _face (not Head_Hide_17_B64C47F3486229273ED8AEA1F530B207) false))

(fn `Load Cal Outfits`
  (returns (Profiles :type "Array of /Game/ModLoaderContent/CharacterReplacer/Profiles/Struct_Outfit Structure"))
  (locals (ProfileArray :type "Array of /Game/ModLoaderContent/CharacterReplacer/Profiles/Struct_Outfit Structure") (TestProfileArray :type "Array of /Game/ModLoaderContent/CharacterReplacer/Profiles/OutfitProfile Class Reference"))
  (`self.PrintToModLoader` "Loading Profiles")
  (`self.GetAllAssets`)
  (for _array_element (`self.Assets`)
    (`self.PrintToModLoader` _array_element)
    (bind _returnvalue (+ (`KismetStringLibrary.FindSubstring` _array_element "/" false true) 1))
    (bind _object (`/Game/Mods/ModLoader/BlueprintLibraries/ModLoaderUtilities.LoadObjectOfClassFromPath` (`KismetStringLibrary.Concat_StrStr` _array_element "." (`KismetStringLibrary.GetSubstring` _array_element _returnvalue (- (`KismetStringLibrary.Len` _array_element) _returnvalue)) "_C") "OutfitProfile_C" self))
    (`/Engine/EditorBlueprintResources/StandardMacros.IsValid` _object
      (:`Is Valid`
        (bind _asoutfit_profile (cast `/Game/ModLoaderContent/CharacterReplacer/Profiles/OutfitProfile` _object)
          (:`CastFailed`
            (`self.PrintToModLoader` "Cast Failed"))))
      (:`Is Not Valid`
        (`self.PrintToModLoader` "Not Valid"))))
  (return (`local.ProfileArray`)))

(fn `Load Cal Profiles`
  (returns (Outfits :type "Array of /Game/ModLoaderContent/CharacterReplacer/Profiles/Struct_UserProfile Structure"))
  (return (`|MakeArray` (struct) :!type "/Game/ModLoaderContent/CharacterReplacer/Profiles/Struct_UserProfile Structure")))

(fn `Load Current Cal Profile`
  (returns (Outfit :type "/Game/ModLoaderContent/CharacterReplacer/Profiles/Struct_UserProfile Structure"))
  (return))

(fn `Replace Body`
  (params (Profile :type "/Game/ModLoaderContent/CharacterReplacer/Profiles/Struct_OutfitPart Structure"))
  (`/Engine/EditorBlueprintResources/StandardMacros.IsValid` Profile_PartMesh_7_3414C82E4CA69032C312AFB783E79B16
    (:`Is Valid`
      (`SkinnedMeshComponent.SetSkinnedAssetAndUpdate` (`Character.Mesh` (`GameplayStatics.GetPlayerCharacter` 0)) Profile_PartMesh_7_3414C82E4CA69032C312AFB783E79B16 false))))

(fn `Replace Cal By Profile`
  (bind (_activeprofile_profilename _activeprofile_outfitref _activeprofile_pants _activeprofile_undershirt _activeprofile_jacket _activeprofile_head _activeprofile_hair _activeprofile_facialhair) (break `/Game/ModLoaderContent/CharacterReplacer/Profiles/Struct_UserProfile` (`self.ActiveProfile`)))
  (`self.Replace Body` _activeprofile_pants)
  (`self.Replace Head` _activeprofile_head)
  (`self.Hide Parts` _activeprofile_pants _activeprofile_undershirt _activeprofile_jacket _activeprofile_head _activeprofile_hair _activeprofile_facialhair))

(fn `Replace Hair`
  (params (Profile :type "/Game/ModLoaderContent/CharacterReplacer/Profiles/Struct_OutfitPart Structure"))
  (`/Engine/EditorBlueprintResources/StandardMacros.IsValid` Profile_PartMesh_7_3414C82E4CA69032C312AFB783E79B16))

(fn `Replace Head`
  (params (Profile :type "/Game/ModLoaderContent/CharacterReplacer/Profiles/Struct_OutfitPart Structure"))
  (`/Engine/EditorBlueprintResources/StandardMacros.IsValid` Profile_PartMesh_7_3414C82E4CA69032C312AFB783E79B16
    (:`Is Valid`
      (bind _face (`self.GetFacialRig` (`GameplayStatics.GetPlayerCharacter` 0)))
      (`SkinnedMeshComponent.SetSkinnedAssetAndUpdate` _face Profile_PartMesh_7_3414C82E4CA69032C312AFB783E79B16 false))))

(fn `Replace Jacket`
  (params (Profile :type "/Game/ModLoaderContent/CharacterReplacer/Profiles/Struct_OutfitPart Structure"))
  (`/Engine/EditorBlueprintResources/StandardMacros.IsValid` Profile_PartMesh_7_3414C82E4CA69032C312AFB783E79B16))

(fn `ResetColor`
  (params (Part :type "/Game/ModLoaderContent/CharacterReplacer/Profiles/Struct_Part Structure (by ref)") (Outfit :type "/Game/ModLoaderContent/CharacterReplacer/Profiles/OutfitProfile Object Reference"))
  (bind _outactors (`GameplayStatics.GetAllActorsOfClass` (`self.CurrentCharacterClass`)))
  (for _array_element _outactors
    (bind (_value _returnvalue) (`BlueprintMapLibrary.Map_Find` (`self.AddonMeshes`) (`KismetStringLibrary.Concat_StrStr` (`KismetSystemLibrary.GetObjectName` _array_element) (`/Game/ModLoaderContent/CharacterReplacer/Profiles/OutfitProfile.GetPartID` Outfit Part))))
    (if _returnvalue
      (bind _skeletalmeshcomponent (`SkeletalMeshActor.SkeletalMeshComponent` _value))
      (for (_array_element_2 _array_index) (`MeshComponent.GetMaterials` _skeletalmeshcomponent)
        (bind _asmaterial_instance_dynamic (cast `MaterialInstanceDynamic` _array_element_2))
        (`PrimitiveComponent.SetMaterial` _skeletalmeshcomponent _array_index (`MaterialInstance.Parent` _asmaterial_instance_dynamic)))
      (`/Game/ModLoaderContent/CharacterReplacer/Profiles/OutfitProfile.OnPartColorReset` Outfit Part))))

(fn `ResetPartVisibility`
  (bind _outactors (`GameplayStatics.GetAllActorsOfClass` (`self.CurrentCharacterClass`)))
  (for _array_element _outactors
    (for _array_element_2 (`self.K2_GetComponentsByClass` _array_element "/Script/Engine.SceneComponent")
      (if (`KismetArrayLibrary.Array_Contains` (`self.HiddenParts`) (`KismetSystemLibrary.GetObjectName` _array_element_2))
        (`SceneComponent.SetVisibility` _array_element_2 true false))))
  (`KismetArrayLibrary.Array_Clear` (`self.HiddenParts`)))

(fn `ResetRotation`
  (`SceneComponent.K2_SetWorldRotation` :`self` (`self.Base`)))

(fn `RotateModel`
  (params (`Pressed?` :type Boolean))
  (if `Pressed?`
    (set `RotatingMovementComponent.RotationRate` (struct :`Yaw` 60.0) (`self.RotatingMovement`))
    (else
      (set `RotatingMovementComponent.RotationRate` (struct) (`self.RotatingMovement`)))))

(fn `Save Cal Profile`
  (params (Outfit :type "/Game/ModLoaderContent/CharacterReplacer/Profiles/Struct_UserProfile Structure"))
  (return))

(fn `Set Active Profile`
  (params (Profile :type "/Game/ModLoaderContent/CharacterReplacer/Profiles/Struct_UserProfile Structure"))
  (set `self.ActiveProfile` Profile)
  (`self.Replace Cal By Profile`))

(fn `SetMeshVisibility`
  (params (MeshComponent :type "SceneComponent Object Reference") (NewVisibility :type Boolean) (PropagateToChildren :type Boolean))
  (bind _hiddenparts (`self.HiddenParts`))
  (bind _outactors (`GameplayStatics.GetAllActorsOfClass` (`self.CurrentCharacterClass`)))
  (for _array_element _outactors
    (for _array_element_2 (`self.K2_GetComponentsByClass` _array_element "/Script/Engine.SceneComponent")
      (bind _returnvalue (`KismetSystemLibrary.GetObjectName` _array_element_2))
      (if (`KismetStringLibrary.EqualEqual_StrStr` _returnvalue (`KismetSystemLibrary.GetObjectName` MeshComponent))
        (`SceneComponent.SetVisibility` _array_element_2 NewVisibility PropagateToChildren)
        (if NewVisibility
          (`KismetArrayLibrary.Array_RemoveItem` _hiddenparts _returnvalue)
          (else
            (`KismetArrayLibrary.Array_AddUnique` _hiddenparts _returnvalue)))))))

(fn `ToggleAllSkeletalMeshes`
  (params (NewVisibility :type Boolean))
  (bind _outactors (`GameplayStatics.GetAllActorsOfClass` (`self.CurrentCharacterClass`)))
  (for _array_element _outactors
    (for _array_element_2 (`SceneComponent.GetChildrenComponents` (`Character.Mesh` _array_element) true)
      (bind _asskeletal_mesh_component (cast `SkeletalMeshComponent` _array_element_2))
      (`self.SetMeshVisibility` _asskeletal_mesh_component NewVisibility))))

(fn `TogglePartVisibility`
  (params (PartType :type "/Game/ModLoaderContent/CharacterReplacer/Profiles/EPartType Enum" :default "NewEnumerator0") (Hidden :type Boolean))
  (bind _returnvalue (not Hidden))
  (bind _outactors (`GameplayStatics.GetAllActorsOfClass` (`self.CurrentCharacterClass`)))
  (for _array_element _outactors
    (bind _asbp_hero (cast `/Game/Characters/Hero/Logic/BP_Hero` _array_element)
      (:`then`
        (`SceneComponent.SetVisibility` (select `/Game/ModLoaderContent/CharacterReplacer/Profiles/EPartType` PartType :`NewEnumerator0` (`/Game/Characters/Hero/Logic/BP_Hero.Pants` _asbp_hero) :`NewEnumerator1` (`/Game/Characters/Hero/Logic/BP_Hero.UnderShirt` _asbp_hero) :`NewEnumerator2` (`/Game/Characters/Hero/Logic/BP_Hero.Jacket` _asbp_hero) :`NewEnumerator3` (`/Game/Characters/Hero/Logic/BP_Hero.face` _asbp_hero) :`NewEnumerator4` (`/Game/Characters/Hero/Logic/BP_Hero.Hair` _asbp_hero) :`NewEnumerator5` (`/Game/Characters/Hero/Logic/BP_Hero.FacialHair` _asbp_hero) :!type "SkinnedMeshComponent Object Reference") _returnvalue false))
      (:`CastFailed`
        (`SceneComponent.SetVisibility` (`Character.Mesh` _array_element) _returnvalue false)))))

(fn `UnequipAll`
  (for _array_element (`self.EquippedOutfits`)
    (for _array_element_2 (`/Game/ModLoaderContent/CharacterReplacer/Profiles/OutfitProfile.Parts` _array_element)
      (`self.UnequipPart` _array_element _array_element_2)))
  (`KismetArrayLibrary.Array_Clear` (`self.EquippedOutfits`)))

(fn `UnequipPart`
  (params (Outfit :type "/Game/ModLoaderContent/CharacterReplacer/Profiles/OutfitProfile Object Reference") (Part :type "/Game/ModLoaderContent/CharacterReplacer/Profiles/Struct_Part Structure"))
  (locals (L_SkeletalActorToRemove :type "SkeletalMeshActor Object Reference") (L_CurrentLoopMesh :type "SkinnedMeshComponent Object Reference"))
  (bind _addonmeshes (`self.AddonMeshes`))
  (`/Engine/EditorBlueprintResources/StandardMacros.IsValid` (`.Mesh_2_5E3D77AC40E797184B5AF79B2C761C03` (break `/Game/ModLoaderContent/CharacterReplacer/Profiles/Struct_Part` Part))
    (:`Is Valid`
      (bind _outactors (`GameplayStatics.GetAllActorsOfClass` (`self.CurrentCharacterClass`)))
      (for _array_element _outactors
        (`|ExecutionSequence`
          (:`then_0`
            (bind _returnvalue (`KismetStringLibrary.Concat_StrStr` (`KismetSystemLibrary.GetObjectName` _array_element) (`/Game/ModLoaderContent/CharacterReplacer/Profiles/OutfitProfile.GetPartID` Outfit Part)))
            (bind (_value _returnvalue_2) (`BlueprintMapLibrary.Map_Find` _addonmeshes _returnvalue))
            (if _returnvalue_2
              (bind _output_get (set `local.L_SkeletalActorToRemove` _value))
              (`BlueprintMapLibrary.Map_Remove` _addonmeshes _returnvalue)
              (`self.K2_DestroyActor` _output_get)))
          (:`then_1`
            (`/Game/ModLoaderContent/CharacterReplacer/Profiles/OutfitProfile.OnPartRemoved` Outfit Outfit Part)
            (`self.OnAnyPartRemoved` Outfit Part)))))))

(fn `UpdateMeshPreview`
  (params (`Skeletal Meshes` :type "SkeletalMeshComponent Object Reference"))
  (bind _scenecapturecomponent2d (`self.SceneCaptureComponent2D`))
  (set `self.Counter` (+ (`self.Counter`) 1))
  (`/Engine/EditorBlueprintResources/StandardMacros.IsValid` (`self.CurrentBP`)
    (:`Is Valid`
      (`self.K2_DestroyActor` (`self.CurrentBP`)))
    (:`Is Not Valid`
      _))
  (bind _returnvalue (`|SpawnActorFromClass` (`self.CurrentCharacterClass`) (`SceneComponent.GetRelativeTransform` (`self.Base`)) "AlwaysSpawn" "OverrideRootScale" null null))
  (bind _output_get (set `self.CurrentBP` _returnvalue))
  (`SceneComponent.K2_AddLocalOffset` _scenecapturecomponent2d (`KismetMathLibrary.MakeVector` 0.0 0.0 (* (`self.Last Mass`) -1.0)) false true)
  (bind _mesh (`Character.Mesh` _returnvalue))
  (bind (_returnvalue_x _returnvalue_y _returnvalue_z) (`KismetMathLibrary.BreakVector` (`PrimitiveComponent.GetCenterOfMass` _mesh "None")))
  (`SceneComponent.K2_AddLocalOffset` _scenecapturecomponent2d (`KismetMathLibrary.MakeVector` 0.0 0.0 _returnvalue_z) false true)
  (set `self.Last Mass` _returnvalue_z)
  (`self.K2_AttachToComponent` _output_get (`self.Base`) "None" "KeepRelative" "KeepRelative" "KeepRelative" true)
  (bind (_returnvalue_roll _returnvalue_pitch _returnvalue_yaw) (`KismetMathLibrary.BreakRotator` (`KismetMathLibrary.FindLookAtRotation` (`SceneComponent.K2_GetComponentLocation` _mesh) (`SceneComponent.K2_GetComponentLocation` (`self.SceneCaptureComponent2D`)))))
  (`SceneComponent.K2_SetWorldRotation` _mesh (`KismetMathLibrary.MakeRotator` 0.0 0.0 (+ _returnvalue_yaw -90.0)) false true))

(fn `UserConstructionScript`)