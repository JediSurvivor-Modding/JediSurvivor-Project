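; Walk mod Blueprint that lets the player hero move slower while a configurable key is held, or toggled on.
; Tick polls raw keys, uses a DoOnce to flip the toggle once per press, and caps nonzero input direction magnitude to the walk ratio by overwriting it.
; Two other keys step that clamped ratio up or down.
; Settings live in a WalkSave object, async-loaded on BeginPlay and created if loading fails.
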(event `self.ReceiveTick`
  (params (DeltaSeconds :type "Float (single-precision)"))
  (bind _returnvalue (`RsGameplayStatics.RsGetPlayerHero`))
  (bind _returnvalue_2 (`GameplayStatics.GetPlayerController` 0))
  (bind _walksaveref (`self.WalkSaveRef`))
  (bind _walksaveref_2 (`self.WalkSaveRef`))
  (bind _walkspeedratio (`/Game/Mods/Walk/WalkSave.WalkSpeedRatio` (`self.WalkSaveRef`)))
  ;[1 0.2414 0 0.11] Tick
  (`|ExecutionSequence`
    (:`then_0`
      (if (`PlayerController.IsInputKeyDown` (`GameplayStatics.GetPlayerController` 0) (`/Game/Mods/Walk/WalkSave.WalkKey` (`self.WalkSaveRef`)))
        ;;[1 1 1] Start Walk
        (`|ExecutionSequence`
          (:`then_0`
            ;;[0.3646 0 0] Toggle Walk
            (`/Engine/EditorBlueprintResources/StandardMacros.DoOnce` false :!label _label
              (:`Completed`
                (set `self.IsActiveWalk` (not (`self.IsActiveWalk`))))))
          (:`then_1`
            ;;[0.2601 1 0.5652] Apply Walk
            (if (> (`rsActor.GetInputDirectionMagnitude` _returnvalue) 0.0) :!label _label_2
              (`rsActor.SetInputDirectionMagnitude` _returnvalue (`/Game/Mods/Walk/WalkSave.WalkSpeedRatio` (`self.WalkSaveRef`))))))
        (else
          ;;[1 1 1] Stop Walking
          (`|ExecutionSequence`
            (:`then_0`
              (goto _label :!via `Reset`))
            (:`then_1`
              (if (and (`self.IsActiveWalk`) (`/Game/Mods/Walk/WalkSave.isToggle` (`self.WalkSaveRef`)))
                (goto _label_2)))))))
    (:`then_1`
      ;;[1 1 1] Change walk Speed multiplier
      (`|ExecutionSequence`
        (:`then_0`
          (if (`PlayerController.WasInputKeyJustPressed` _returnvalue_2 (`/Game/Mods/Walk/WalkSave.IncreaseSpeedKey` _walksaveref_2))
            (set `/Game/Mods/Walk/WalkSave.WalkSpeedRatio` (`KismetMathLibrary.FClamp` (+ _walkspeedratio 0.1) 0.2) _walksaveref)))
        (:`then_1`
          (if (`PlayerController.WasInputKeyJustPressed` _returnvalue_2 (`/Game/Mods/Walk/WalkSave.DecreaseSpeedKey` _walksaveref_2))
            (set `/Game/Mods/Walk/WalkSave.WalkSpeedRatio` (`KismetMathLibrary.FClamp` (+ _walkspeedratio -0.1) 0.2) _walksaveref)))))))

(event `self.ReceiveBeginPlay`
  ;[0.1521 0.477 1 0.232] Load and Save
  (`self.LoadWalkConfigs`))

(event `SaveWalkConfigs`
  ;[0.1521 0.477 1 0.232] Load and Save
  (`self.WalkSaveRef`
    (:`then`
      _)
    (:`else`
      (bind _returnvalue (`GameplayStatics.CreateSaveGameObject` "/Game/Mods/Walk/WalkSave.WalkSave_C"))
      (set `self.WalkSaveRef` _returnvalue)))
  (`GameplayStatics.SaveGameToSlot` (`self.WalkSaveRef`) "WalkSave"))

(event `LoadWalkConfigs`
  ;[0.1521 0.477 1 0.232] Load and Save
  (bind (_savegame _bsuccess) (`AsyncActionHandleSaveGame.AsyncLoadGameFromSlot` "WalkSave")
    (:`Completed`
      (if _bsuccess
        (bind _aswalk_save (cast `/Game/Mods/Walk/WalkSave` _savegame))
        (set `self.WalkSaveRef` _aswalk_save)
        (else
          (`self.SaveWalkConfigs`))))))

(fn `UserConstructionScript`)